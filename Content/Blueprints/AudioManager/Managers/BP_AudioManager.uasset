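; Audio manager Blueprint that plays 2D sound effects and an indexed list of music tracks, with sounds set to persist across level transitions.
; Effect playback stores only the latest component, which the kill event fades out instantly before printing a debug message.
; Music fades in the current track, while TransitionSong advances only if that asset's total duration is at most half a second, fading out and playing the next without index wrapping.
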(event Custom|PlaySoundEffect
  (params (Sound%20Effect :type Sound%20Base%20Object%20Reference))
  ;[0.15 0.15 0.15 0.5] Sound Effects
  ;;[0.15 0.15 0.15 0.5] Play Sound Effects
  (bind _returnvalue (Audio|SpawnSound2D Sound%20Effect 1.5 1.0 0.0 0 true false))
  (Variables|Default|SetSavedSoundTest _returnvalue))

(event Custom|KillSoundEffect
  ;[0.15 0.15 0.15 0.5] Sound Effects
  ;;[0.15 0.15 0.15 0.5] Kill Sound Effects
  (Audio|Components|Audio|FadeOut (Variables|Default|GetSavedSoundTest) 0.0 0.0 "Linear" :!class /Script/Engine.AudioComponent)
  (Development|PrintString "Hello"))

(event Custom|PlayMusic
  (bind _returnvalue (Audio|SpawnSound2D (Utilities|Array|Get(acopy) (Variables|Default|GetMusicLoopList) (Variables|Default|GetCurrentSong)) 1.0 1.0 0.0 0 true false))
  (Audio|Components|Audio|FadeIn _returnvalue 0.25 1.0 0.0 "Linear" :!class /Script/Engine.AudioComponent)
  (Variables|Default|SetActiveSong _returnvalue))

(event Custom|TransitionSong
  (if (<= (Variables|/Script/Engine.SoundBase|GetDuration (Utilities|Array|Get(acopy) (Variables|Default|GetMusicLoopList) (Variables|Default|GetCurrentSong))) 0.5)
    (Audio|Components|Audio|FadeOut (Variables|Default|GetActiveSong) 0.5 0.0 "Linear" :!class /Script/Engine.AudioComponent)
    (Variables|Default|SetCurrentSong (+ (Variables|Default|GetCurrentSong) 1))
    (CallFunction|PlayMusic)))

(fn ConstructionScript)