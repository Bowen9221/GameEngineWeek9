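; BP_ObjectPool is an object pool actor that pre-spawns PoolSize instances of PooledClass on BeginPlay for reuse.
; Each BP_PooledActor gets its owner set, receives a despawn message and joins Pool and Available.
; GetPooledActor is meant to pop, move and wake an actor, but its Length < 0 check never passes.
; ReturnActor despawns, attaches and requeues actors, while Despawn requeues but disables the pool itself, not InActor.
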(event EventBeginPlay
  (CallFunction|InitializePool))

(fn ConstructionScript)

(fn InitializePool
  (for _index (range 0 (- (Variables|Default|GetPoolSize) 1))
    (bind _returnvalue (Game|SpawnActorfromClass (Variables|Default|GetPooledClass) (Transformation|GetActorTransform) "Undefined" "MultiplyWithRoot" 0 0))
    (bind _asbp_pooled_actor (Utilities|Casting|CastToBP_PooledActor _returnvalue))
    (Variables|/Game/Blueprints/ObjectPooling/BP_PooledActor.BP_PooledActor_C|Setpool%20Owner _asbp_pooled_actor self)
    (Class|BPIPooled|OnDespawned(Message) _returnvalue)
    (Utilities|Array|Add (Variables|Default|GetPool) _returnvalue)
    (Utilities|Array|Add (Variables|Default|GetAvailable) _returnvalue)))

(fn GetPooledActor
  (params (SpawnTransform :type Transform))
  (bind _available (Variables|Default|GetAvailable))
  (bind _returnvalue (Utilities|Array|Length _available))
  (if (< _returnvalue 0)
    (Variables|Default|SetResult%20Actor (Utilities|Array|Get(acopy) _available (Utilities|Array|LastIndex _available)))
    (Utilities|Array|RemoveIndex _available (- _returnvalue 1))
    (Utilities|IsValid (Variables|Default|GetResult%20Actor)
      (:Is%20Valid
        (Transformation|DetachFromActor (Variables|Default|GetResult%20Actor) "KeepRelative" "KeepRelative" "KeepRelative")
        (Transformation|SetActorTransform (Variables|Default|GetResult%20Actor) SpawnTransform)
        (Class|BPIPooled|OnSpawned(Message) (Variables|Default|GetResult%20Actor)))
      (:Is%20Not%20Valid
        _))
    (return (Variables|Default|GetResult%20Actor))))

(fn ReturnActor
  (params (ReturnActor :type Actor%20Object%20Reference))
  (Utilities|IsValid ReturnActor
    (:Is%20Valid
      (Class|BPIPooled|OnDespawned(Message) ReturnActor)
      (Transformation|AttachActorToActor ReturnActor self "None" "KeepRelative" "KeepRelative" "KeepRelative" true)
      (Utilities|Array|Add (Variables|Default|GetAvailable) ReturnActor))))

(fn Despawn
  (params (InActor :type Actor%20Object%20Reference))
  (if (Utilities|IsValid InActor)
    (Rendering|SetActorHiddenInGame true)
    (Collision|SetActorEnableCollision false)
    (Actor|Tick|SetActorTickEnabled false)
    (Utilities|Array|Add (Variables|Default|GetAvailable) InActor)))