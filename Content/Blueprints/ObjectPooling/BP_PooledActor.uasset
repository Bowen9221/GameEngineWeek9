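; Base pooled actor for an object pooling system that toggles between active and dormant states instead of being destroyed.
; OnSpawned shows the actor, enables collision and tick, marks it in use and restarts a lifetime timer.
; When the timer fires, AutoReturn calls ReturnToPool.
; OnDespawned hides the actor, disables collision and tick, clears the in-use flag and cancels the timer.
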(event Custom|AutoReturn
  ;[0.15 0.15 0.15 0.5] Enable Actor
  ;;[0.15 0.15 0.15 0.5] Returns Object To Pool
  (CallFunction|ReturntoPool))

(event EventOnSpawned
  ;[0.15 0.15 0.15 0.5] Enable Actor
  (Rendering|SetActorHiddenInGame false)
  (Collision|SetActorEnableCollision true)
  (Actor|Tick|SetActorTickEnabled true)
  (Variables|Default|SetBinUse true)
  (Utilities|Time|ClearandInvalidateTimerbyHandle (Variables|Default|GetLifeTimer))
  (Utilities|Time|SetTimerbyFunctionName 0 "AutoReturn" (Variables|Default|GetLifetime)))

(event EventOnDespawned
  (Rendering|SetActorHiddenInGame true)
  (Collision|SetActorEnableCollision false)
  (Actor|Tick|SetActorTickEnabled false)
  (Variables|Default|SetBinUse false)
  (Utilities|Time|ClearandInvalidateTimerbyHandle (Variables|Default|GetLifeTimer)))

(fn ConstructionScript)